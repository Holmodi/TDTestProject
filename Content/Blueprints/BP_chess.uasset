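; Board cell actor for a tic-tac-toe game that forwards clicks with its Index to BP_TicTacGameMode as player input.
; It binds to the game mode's begin and view-update events, turning white when a game begins.
; On updates it reads its own board entry and applies a random X or O material only while still white, so the chosen look stays fixed.
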(event `self.ReceiveBeginPlay`
  (`PrimitiveComponent.SetMaterial` (`self.StaticMesh`) 0 "/Game/Material/M_1_1.M_1_1")
  (bind _asbp_tic_tac_game_mode (cast `/Game/Blueprints/BP_TicTacGameMode` (`GameplayStatics.GetGameMode`)))
  (bind _output_get (set `self.As BP Tic Tac Game Mode` _asbp_tic_tac_game_mode))
  (add `TicTacGameMode.OnGameBegin` _output_get (delegate `OnGameBegin_Event_0`))
  (add `TicTacGameMode.OnGameUpdateView` _output_get (delegate `OnGameUpdateView_Event`)))

(event `OnGameBegin_Event_0`
  (`PrimitiveComponent.SetMaterial` (`self.StaticMesh`) 0 "/Game/Material/M_White.M_White")
  (set `self.CurrentMaterial` "/Game/Material/M_White.M_White"))

(event `OnGameUpdateView_Event`
  (params (BoardCells :type "Array of EPlayerMark Enum (by ref)"))
  (`self.UpdateView` BoardCells))

(event `self.ReceiveActorOnClicked`
  (params (ButtonPressed :type "Key Structure"))
  (`TicTacGameMode.PlayerInput` (`self.As BP Tic Tac Game Mode`) (`self.Index`)))

(fn `ResetMaterial`
  (`PrimitiveComponent.SetMaterial` (`self.StaticMesh`) 0 null))

(fn `UpdateView`
  (params (Array :type "Array of EPlayerMark Enum"))
  (if (== (`self.CurrentMaterial`) "/Game/Material/M_White.M_White")
    (switch `EPlayerMark` (`|GetArrayItem` Array (`self.Index`))
      (:`Empty`
        (set `self.CurrentMaterial` "/Game/Material/M_White.M_White"))
      (:`PlayerX`
        (set `self.CurrentMaterial` (`KismetArrayLibrary.Array_Random` (`self.X_Materials`))))
      (:`PlayerO`
        (bind _output_get (set `self.CurrentMaterial` (`KismetArrayLibrary.Array_Random` (`self.O_Materials`))))))
    (`PrimitiveComponent.SetMaterial` (`self.StaticMesh`) 0 _output_get)))

(fn `UserConstructionScript`)